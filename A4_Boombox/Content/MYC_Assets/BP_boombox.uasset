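; Interactive boombox actor that the player can switch on and off when standing near it.
; Entering or leaving the box collider adds or removes an Enhanced Input mapping context, so the interact action only works in proximity.
; The action drives a FlipFlop that swaps the display material, plays or stops music, and starts or stops a timeline animating both speakers' X offset.
; Debug messages print on overlap and input.
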(event OnComponentBeginOverlap(BoxCollider)
  (params (OverlappedComponent :type Primitive%20Component%20Object%20Reference) (OtherActor :type Actor%20Object%20Reference) (OtherComp :type Primitive%20Component%20Object%20Reference) (OtherBodyIndex :type Integer) (bFromSweep :type Boolean) (SweepResult :type Hit%20Result%20Structure%20%28by%20ref%29))
  (Development|PrintString (Utilities|String|Append "Player " (Utilities|GetDisplayName OtherActor) " is near Boombox") true true "(R=0.000000,G=0.660000,B=1.000000,A=1.000000)" 5.0)
  ;[1 1 1] Enable Input Interaction
  (Input|AddMappingContext (PlayerController|LocalPlayerSubsystems|GetEnhancedInputLocalPlayerSubsystem (Game|GetPlayerController 0)) "/Game/Inputs/IMC_Boombox.IMC_Boombox" 0 "(bIgnoreAllPressedKeysUntilRelease=True,bForceImmediately=False,bNotifyUserSettings=False)"))

(event OnComponentEndOverlap(BoxCollider)
  (params (OverlappedComponent :type Primitive%20Component%20Object%20Reference) (OtherActor :type Actor%20Object%20Reference) (OtherComp :type Primitive%20Component%20Object%20Reference) (OtherBodyIndex :type Integer))
  (Development|PrintString (Utilities|String|Append "Player " (Utilities|GetDisplayName OtherActor) " moved away from Boombox") true true "(R=0.000000,G=0.660000,B=1.000000,A=1.000000)" 5.0)
  ;[1 1 1] Disable Input Interaction
  (Input|RemoveMappingContext (PlayerController|LocalPlayerSubsystems|GetEnhancedInputLocalPlayerSubsystem (Game|GetPlayerController 0)) "/Game/Inputs/IMC_Boombox.IMC_Boombox" "(bIgnoreAllPressedKeysUntilRelease=True,bForceImmediately=False,bNotifyUserSettings=False)"))

(event Input|EnhancedActionEvents|EnhancedInputActionIA_Boombox_Proximity
  (params (ActionValue :type Boolean) (ElapsedSeconds :type Float%20%28double-precision%29) (TriggeredSeconds :type Float%20%28double-precision%29) (InputAction :type Input%20Action%20Object%20Reference :default "/Game/Inputs/IA_Boombox_Proximity.IA_Boombox_Proximity"))
  (bind _speaker_r (Variables|Default|GetSpeaker_R))
  (bind _speaker_l (Variables|Default|GetSpeaker_L))
  (bind _music (Variables|Default|GetMusic))
  (bind _relativelocation (Variables|/Script/Engine.SceneComponent|GetRelativeLocation _speaker_r))
  (bind _relativelocation_2 (Variables|/Script/Engine.SceneComponent|GetRelativeLocation _speaker_l))
  (bind (_x _y _z) (Math|Vector|BreakVector _relativelocation))
  (bind (_x_2 _y_2 _z_2) (Math|Vector|BreakVector _relativelocation_2))
  (:Started
    (Development|PrintString "Started: Player is NEAR Boombox and pressed the Input Action Key" true true "(R=0.000000,G=1.000000,B=0.070262,A=1.000000)" 5.0)
    (Utilities|FlowControl|FlipFlop
      (:A
        ;[1 1 1] Toggle Boombox Playing ON
        (Rendering|Material|SetMaterial (Variables|Default|GetDisplay) 0 "/Engine/MapTemplates/Materials/BasicAsset03.BasicAsset03")
        (Audio|Components|Audio|Play _music 0.0)
        ;;[1 1 1] Speakers Animation
        (bind _position_offset (Timeline|Timeline%20Speakers Play)
          (:Update
            (Transformation|SetRelativeLocation _speaker_r (Math|Vector|MakeVector _position_offset _y _z) false false)
            (Transformation|SetRelativeLocation _speaker_l (Math|Vector|MakeVector _position_offset _y_2 _z_2) false false))))
      (:B
        ;[1 1 1] Toggle Boombox Playing OFF
        (Rendering|Material|SetMaterial (Variables|Default|GetDisplay) 0 "/Engine/MapTemplates/Materials/BasicAsset01.BasicAsset01")
        (Audio|Components|Audio|Stop _music)
        (Timeline|Timeline%20Speakers Stop)))))

(event Collision|EventActorBeginOverlap
  (params (OtherActor :type Actor%20Object%20Reference)))

(event EventTick
  (params (DeltaSeconds :type Float%20%28single-precision%29)))

(fn ConstructionScript)